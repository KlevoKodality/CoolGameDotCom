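; BP_TrainingActor is a training dummy that reports incoming hits as green on-screen debug text in Russian.
; BeginPlay casts the player pawn to BP_TopDownCharacter and caches it.
; On AnyDamage, it prints the player's equipped weapon damage multiplied by that weapon's buff, ignoring the event's actual damage value and causer.
; It tracks no health and has no other active logic.
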(event `self.ReceiveAnyDamage`
  (params (Damage :type "Float (single-precision)") (DamageType :type "DamageType Object Reference") (InstigatedBy :type "Controller Object Reference") (DamageCauser :type "Actor Object Reference"))
  (bind _equippedweapon (`/Game/TopDown/Blueprints/BP_TopDownCharacter.EquippedWeapon` (stale `self.ReceiveBeginPlay` _output_get)))
  (`KismetSystemLibrary.PrintString` (`KismetStringLibrary.Concat_StrStr` "Манекен получил урон: " (`KismetStringLibrary.Conv_DoubleToString` (* (`ABaseMeleeWeapon.WeaponDamage` _equippedweapon) (`ABaseMeleeWeapon.WeaponBuff` _equippedweapon)))) true true (struct :`R` 0.223111 :`G` 1.0 :`A` 1.0)))

(event `self.ReceiveBeginPlay`
  (bind _asbp_top_down_character (cast `/Game/TopDown/Blueprints/BP_TopDownCharacter` (`GameplayStatics.GetPlayerPawn` 0)))
  (bind _output_get (set `self.As BP Top Down Character` _asbp_top_down_character)))

(fn `UserConstructionScript`)