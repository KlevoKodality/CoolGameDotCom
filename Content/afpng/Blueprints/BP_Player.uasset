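; BP_Player is the player character, handling WASD movement and a dash on Space bar.
; Key events set a flag per direction, which Tick reads to add movement input along fixed world axes, independent of camera.
; Space calls PerformDash, whose logic is not defined in this graph.
; A separate custom event, not called here, spawns a particle effect at the character's last update location and destroys it after a short delay.
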(event `CustomEvent`
  (bind _returnvalue (`GameplayStatics.SpawnEmitterAtLocation` "/Engine/Tutorial/SubEditors/TutorialAssets/TutorialParticleSystem.TutorialParticleSystem" (`CharacterMovementComponent.GetLastUpdateLocation` (`self.CharacterMovement`))))
  (`KismetSystemLibrary.Delay` 0.2)
  (`ActorComponent.K2_DestroyComponent` _returnvalue))

(event `Key|SpaceBar`
  (params (Key :type "Key Structure"))
  (:`Pressed`
    (`self.PerformDash`)))

(event `Key|W`
  (params (Key :type "Key Structure"))
  (:`Pressed`
    (set `self.W` true))
  (:`Released`
    (set `self.W` false)))

(event `Key|S`
  (params (Key :type "Key Structure"))
  (:`Pressed`
    (set `self.S` true))
  (:`Released`
    (set `self.S` false)))

(event `self.ReceiveTick`
  (params (DeltaSeconds :type "Float (single-precision)"))
  (`|ExecutionSequence`
    (:`then_0`
      (if (`self.W`)
        (`self.AddMovementInput` (1.0 0.0 0.0))))
    (:`then_1`
      (if (`self.A`)
        (`self.AddMovementInput` (0.0 -1.0 0.0))))
    (:`then_2`
      (if (`self.S`)
        (`self.AddMovementInput` (-1.0 0.0 0.0))))
    (:`then_3`
      (if (`self.D`)
        (`self.AddMovementInput` (0.0 1.0 0.0))))))

(event `Key|A`
  (params (Key :type "Key Structure"))
  (:`Pressed`
    (set `self.A` true))
  (:`Released`
    (set `self.A` false)))

(event `Key|D`
  (params (Key :type "Key Structure"))
  (:`Pressed`
    (set `self.D` true))
  (:`Released`
    (set `self.D` false)))

(fn `UserConstructionScript`)